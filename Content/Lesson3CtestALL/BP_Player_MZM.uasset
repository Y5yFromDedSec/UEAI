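; Player character Blueprint with Enhanced Input handlers for camera-relative movement, look, grounded jump, sprint and a montage-based dodge.
; Sprint needs a hold, movement input and clear state flags, then changes walk speed, animation play rate (via interface) and timeline-lerped spring arm length.
; Debug keys M, N and X toggle an enemy's AI between Passive and Attack, make noise with an explosion effect, and report damage for AI perception.
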(event `self.ReceiveBeginPlay`)

(event `self.ReceiveActorBeginOverlap`
  (params (OtherActor :type "Actor Object Reference")))

(event `EnhancedInput|/Game/Lesson3CtestALL/IA_MZM/IA_Move_MZM`
  (params (ActionValue :type "Vector2D Structure") (ElapsedSeconds :type "Float (double-precision)") (TriggeredSeconds :type "Float (double-precision)") (InputAction :type "InputAction Object Reference" :default "/Game/Lesson3CtestALL/IA_MZM/IA_Move_MZM.IA_Move_MZM"))
  (bind (_returnvalue_roll _returnvalue_pitch _returnvalue_yaw) (`KismetMathLibrary.BreakRotator` (`self.GetControlRotation`)))
  (bind (_x _y) (`KismetMathLibrary.BreakVector2D` ActionValue))
  ;[1 1 1] 玩家角色移动
  (:`Triggered`
    (set `self.OriginForward` _x) ; 当按下移动键时设置初始前进方向
    (set `self.OriginRight` _y) ; 当按下移动键时设置初始右进方向
    (`self.AddMovementInput` (`KismetMathLibrary.GetForwardVector` (`KismetMathLibrary.MakeRotator` 0.0 0.0 _returnvalue_yaw)) (`self.OriginForward`)) ; WS控制前进后退
    (`self.AddMovementInput` (`KismetMathLibrary.GetRightVector` (`KismetMathLibrary.MakeRotator` 0.0 0.0 _returnvalue_yaw)) (`self.OriginRight`)) ; AD控制左右移动
  )
  (:`Canceled`
    (set `self.OriginForward` 0.0 :!label _label) ; 当完成or取消时将初始前进方向设置为0
    (set `self.OriginRight` 0.0) ; 当完成or取消时将初始右进方向设置为0
  )
  (:`Completed`
    (goto _label)))

(event `self.ReceiveTick`
  (params (DeltaSeconds :type "Float (single-precision)")))

(event `EnhancedInput|/Game/Lesson3CtestALL/IA_MZM/IA_CameraControl_MZM`
  (params (ActionValue :type "Vector2D Structure") (ElapsedSeconds :type "Float (double-precision)") (TriggeredSeconds :type "Float (double-precision)") (InputAction :type "InputAction Object Reference" :default "/Game/Lesson3CtestALL/IA_MZM/IA_CameraControl_MZM.IA_CameraControl_MZM"))
  (bind (_x _y) (`KismetMathLibrary.BreakVector2D` ActionValue))
  ;[1 1 1] 相机控制
  (:`Triggered`
    (`self.AddControllerYawInput` _x) ; X为屏幕横轴，控制水平方向
    (`self.AddControllerPitchInput` (* _y -1.0)) ; Y轴为屏幕竖轴，控制垂直方向
  ))

(event `EnhancedInput|/Game/Lesson3CtestALL/IA_MZM/IA_Sprint_MZM`
  (params (ActionValue :type Boolean) (ElapsedSeconds :type "Float (double-precision)") (TriggeredSeconds :type "Float (double-precision)") (InputAction :type "InputAction Object Reference" :default "/Game/Lesson3CtestALL/IA_MZM/IA_Sprint_MZM.IA_Sprint_MZM"))
  ;[1 1 1] 冲刺逻辑
  (:`Triggered`
    (`self.CanSprinting` ElapsedSeconds ; 冲刺的状态判断
      (:`满足冲刺`
        (`self.Start Sprinting`) ; 我他妈来了
      )
      (:`不满足冲刺`
        (`self.End Sprinting`) ; 萎了
      )))
  (:`Completed`
    (if (`self.isSprinting`)
      (`self.End Sprinting`) ; 萎了
    )))

(event `ChangeCameraBoomLength`
  (params (`increase?` :type Boolean))
  ;[1 1 1] 相机效果
  (if `increase?`
    (bind (_direction _alpha) (`Timeline|时间轴` :!label _label_2) ; 0.5内变化0-1
      (:`Update`
        (set `SpringArmComponent.TargetArmLength` (`KismetMathLibrary.Lerp` 310.0 450.0 _alpha) (`self.SpringArm`)) ; 每帧更新长度
      ))
    (else
      (goto _label_2 :!via `Reverse`))))

(event `EnhancedInput|/Game/Lesson3CtestALL/IA_MZM/IA_Jump_MZM`
  (params (ActionValue :type Boolean) (ElapsedSeconds :type "Float (double-precision)") (TriggeredSeconds :type "Float (double-precision)") (InputAction :type "InputAction Object Reference" :default "/Game/Lesson3CtestALL/IA_MZM/IA_Jump_MZM.IA_Jump_MZM"))
  ;[1 1 1] 跳跃逻辑
  (:`Triggered`
    (if (`NavMovementComponent.IsMovingOnGround` (`self.CharacterMovement`))
      (`self.Jump`) ; 芜湖起飞！
    )))

(event `EnhancedInput|/Game/Lesson3CtestALL/IA_MZM/IA_Dodge_MZM`
  (params (ActionValue :type Boolean) (ElapsedSeconds :type "Float (double-precision)") (TriggeredSeconds :type "Float (double-precision)") (InputAction :type "InputAction Object Reference" :default "/Game/Lesson3CtestALL/IA_MZM/IA_Dodge_MZM.IA_Dodge_MZM"))
  (:`Completed`
    (`AnimInstance.Montage_Play` (`SkeletalMeshComponent.GetAnimInstance` (`self.Mesh`)) "/Game/Lesson3CtestALL/Anime_MZM/Dodge_MZM/GreatSword_Dodge_F1_Montage_MZM.GreatSword_Dodge_F1_Montage_MZM" 1.5 "MontageLength" 0.0 true)
    (`KismetSystemLibrary.PrintString` "我在翻滚！")))

(event `Key|M`
  (params (Key :type "Key Structure"))
  (:`Pressed`
    (`KismetSystemLibrary.PrintString` "改变AI状态") ; Debug
    (bind _returnvalue (`GameplayStatics.GetActorOfClass` "/Game/M_Enemy/BP_EnemyBase_MZM.BP_EnemyBase_MZM_C")) ; 获取Actor类
    (bind _asaic_enemy_base_mzm (cast `/Game/M_Enemy/AI/AIC_Enemy_Base_MZM` (`AIBlueprintHelperLibrary.GetAIController` _returnvalue))) ; 将AIC转化为我们的AIC
    (`/Engine/EditorBlueprintResources/StandardMacros.FlipFlop` ; 翻转！
      (:`A`
        (`/Game/M_Enemy/AI/AIC_Enemy_Base_MZM.SetStatesAsPassive` _asaic_enemy_base_mzm) ; 切换为Passive
      )
      (:`B`
        (`/Game/M_Enemy/AI/AIC_Enemy_Base_MZM.SetStatesAsAttack` _asaic_enemy_base_mzm self) ; 切换为Attack
      ))))

(event `Key|N`
  (params (Key :type "Key Structure"))
  (bind _returnvalue (`self.K2_GetActorLocation`))
  (:`Pressed`
    (`self.MakeNoise` 1.0 self _returnvalue)
    (`GameplayStatics.SpawnEmitterAtLocation` "/Game/StarterContent/Particles/P_Explosion.P_Explosion" _returnvalue)
    (`GameplayStatics.PlaySoundAtLocation` "/Game/StarterContent/Audio/Explosion01.Explosion01" _returnvalue (struct) 1.0 1.0 0.0 null null null null)))

(event `Key|X`
  (params (Key :type "Key Structure"))
  (:`Pressed`
    (bind _returnvalue (`GameplayStatics.GetActorOfClass` "/Game/M_Enemy/BP_EnemyBase_MZM.BP_EnemyBase_MZM_C"))
    (`AISense_Damage.ReportDamageEvent` _returnvalue self 0.0 (`self.K2_GetActorLocation`))))

(fn `End Sprinting`
  (set `CharacterMovementComponent.MaxWalkSpeed` 600.0 (`self.CharacterMovement`)) ; 设置最大速度
  (message `/Game/Lesson3CtestALL/BPI/BPI_Anime.INT_SetPlayRate` (`SkeletalMeshComponent.GetAnimInstance` (`self.Mesh`)) 1.0) ; 调用接口去设置播放速率
  (set `self.isSprinting` false) ; 记录玩家处于非冲刺状态
  (`self.ChangeCameraBoomLength` false) ; 缩短相机臂
)

(fn `Start Sprinting`
  (set `CharacterMovementComponent.MaxWalkSpeed` 800.0 (`self.CharacterMovement`)) ; 设置最大速度
  (message `/Game/Lesson3CtestALL/BPI/BPI_Anime.INT_SetPlayRate` (`SkeletalMeshComponent.GetAnimInstance` (`self.Mesh`)) 1.5) ; 调用接口去设置播放速率
  (set `self.isSprinting` true) ; 记录玩家处于冲刺状态
  (`self.ChangeCameraBoomLength` true) ; 伸长相机臂
)

(fn `UserConstructionScript`)