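; Player character Blueprint for melee combat with a socket-attached greatsword, handling movement, camera, sprint, jump, dodge, combo light attacks and charged heavy attacks.
; Check macros gate actions on state flags, with stamina costs for attacks and rolls; interface events reset states and take damage.
; Weapon hits use timer-driven sphere sweeps between previous and current sword socket positions, damaging each actor once per swing.
; Debug keys exercise enemy AI and perception; stamina recovery is stubbed.
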(event `self.ReceiveBeginPlay`
  (`/Game/Lesson3CtestALL/Player_BaseData.InitAllValue` (`self.Player_BaseData`))
  (`self.SpawnSword`))

(event `self.ReceiveActorBeginOverlap`
  (params (OtherActor :type "Actor Object Reference")))

(event `self.ReceiveTick`
  (params (DeltaSeconds :type "Float (single-precision)")))

(event `SpawnSword`
  ;[1 1 1] 自定义事件：武器生成
  (bind _returnvalue (`|SpawnActorFromClass` "/Game/Lesson3CtestALL/Weapon/BP_MyGreatSword_00.BP_MyGreatSword_00_C" (`self.GetTransform`) "Undefined" "MultiplyWithRoot" null null)) ; 生成哪吧武器，必须是蓝图类
  (`self.K2_AttachToComponent` _returnvalue (`self.Mesh`) "myGreatSword" "SnapToTarget" "SnapToTarget" "SnapToTarget" true) ; 再对象的哪里生成
)

(event `Key|M`
  (params (Key :type "Key Structure"))
  ;[1 1 1] AI验证模块
  (:`Pressed`
    (`KismetSystemLibrary.PrintString` "改变AI状态") ; Debug
    (bind _returnvalue (`GameplayStatics.GetActorOfClass` "/Game/M_Enemy/BP_EnemyBase_MZM.BP_EnemyBase_MZM_C")) ; 获取Actor类
    (bind _asaic_enemy_base_mzm (cast `/Game/M_Enemy/AI/AIC_Enemy_Base_MZM` (`AIBlueprintHelperLibrary.GetAIController` _returnvalue))) ; 将AIC转化为我们的AIC
    (`/Engine/EditorBlueprintResources/StandardMacros.FlipFlop` ; 翻转！
      (:`A`
        (`/Game/M_Enemy/AI/AIC_Enemy_Base_MZM.SetStatesAsPassive` _asaic_enemy_base_mzm) ; 切换为Passive
      )
      (:`B`
        (`/Game/M_Enemy/AI/AIC_Enemy_Base_MZM.SetStatesAsAttack` _asaic_enemy_base_mzm self) ; 切换为Attack
      ))))

(event `EnhancedInput|/Game/Lesson3CtestALL/IA_MZM/IA_Move_MZM`
  (params (ActionValue :type "Vector2D Structure") (ElapsedSeconds :type "Float (double-precision)") (TriggeredSeconds :type "Float (double-precision)") (InputAction :type "InputAction Object Reference" :default "/Game/Lesson3CtestALL/IA_MZM/IA_Move_MZM.IA_Move_MZM"))
  (bind (_returnvalue_roll _returnvalue_pitch _returnvalue_yaw) (`KismetMathLibrary.BreakRotator` (`self.GetControlRotation`)))
  (bind (_x _y) (`KismetMathLibrary.BreakVector2D` ActionValue))
  ;[1 1 1] 玩家角色移动
  (:`Triggered`
    (set `self.OriginForward` _x) ; 当按下移动键时设置初始前进方向
    (set `self.OriginRight` _y) ; 当按下移动键时设置初始右进方向
    (`self.AddMovementInput` (`KismetMathLibrary.GetForwardVector` (`KismetMathLibrary.MakeRotator` 0.0 0.0 _returnvalue_yaw)) (`self.OriginForward`)) ; WS控制前进后退
    (`self.AddMovementInput` (`KismetMathLibrary.GetRightVector` (`KismetMathLibrary.MakeRotator` 0.0 0.0 _returnvalue_yaw)) (`self.OriginRight`)) ; AD控制左右移动
  )
  (:`Canceled`
    (set `self.OriginForward` 0.0 :!label _label) ; 当完成or取消时将初始前进方向设置为0
    (set `self.OriginRight` 0.0) ; 当完成or取消时将初始右进方向设置为0
  )
  (:`Completed`
    (goto _label)))

(event `StartSPRecover`
  (`KismetSystemLibrary.RetriggerableDelay` 1.5)
  (`KismetSystemLibrary.K2_SetTimerDelegate` (delegate `SPCostRecoverLoop`) 0.1 true))

(event `Key|N`
  (params (Key :type "Key Structure"))
  (bind _returnvalue (`self.K2_GetActorLocation`))
  ;[1 1 1] AI验证模块
  (:`Pressed`
    (`self.MakeNoise` 1.0 self _returnvalue)
    (`GameplayStatics.SpawnEmitterAtLocation` "/Game/StarterContent/Particles/P_Explosion.P_Explosion" _returnvalue)
    (`GameplayStatics.PlaySoundAtLocation` "/Game/StarterContent/Audio/Explosion01.Explosion01" _returnvalue (struct) 1.0 1.0 0.0 null null null null)))

(event `SPCostRecoverLoop`
  (if true
    _))

(event `EnhancedInput|/Game/Lesson3CtestALL/IA_MZM/IA_CameraControl_MZM`
  (params (ActionValue :type "Vector2D Structure") (ElapsedSeconds :type "Float (double-precision)") (TriggeredSeconds :type "Float (double-precision)") (InputAction :type "InputAction Object Reference" :default "/Game/Lesson3CtestALL/IA_MZM/IA_CameraControl_MZM.IA_CameraControl_MZM"))
  (bind (_x _y) (`KismetMathLibrary.BreakVector2D` ActionValue))
  ;[1 1 1] 相机控制
  (:`Triggered`
    (`self.AddControllerYawInput` _x) ; X为屏幕横轴，控制水平方向
    (`self.AddControllerPitchInput` (* _y -1.0)) ; Y轴为屏幕竖轴，控制垂直方向
  ))

(event `Key|X`
  (params (Key :type "Key Structure"))
  ;[1 1 1] AI验证模块
  (:`Pressed`
    (bind _returnvalue (`GameplayStatics.GetActorOfClass` "/Game/M_Enemy/BP_EnemyBase_MZM.BP_EnemyBase_MZM_C"))
    (`AISense_Damage.ReportDamageEvent` _returnvalue self 0.0 (`self.K2_GetActorLocation`))))

(event `EnhancedInput|/Game/Lesson3CtestALL/IA_MZM/IA_Sprint_MZM`
  (params (ActionValue :type Boolean) (ElapsedSeconds :type "Float (double-precision)") (TriggeredSeconds :type "Float (double-precision)") (InputAction :type "InputAction Object Reference" :default "/Game/Lesson3CtestALL/IA_MZM/IA_Sprint_MZM.IA_Sprint_MZM"))
  ;[1 1 1] 冲刺逻辑
  (:`Triggered`
    (`self.CanSprinting` ElapsedSeconds ; 冲刺的状态判断
      (:`满足冲刺`
        (`self.Start Sprinting`) ; 我他妈来了
      )
      (:`不满足冲刺`
        (`self.End Sprinting`) ; 萎了
      )))
  (:`Completed`
    (if (`self.isSprinting`)
      (`self.End Sprinting`) ; 萎了
    )))

(event `ChangeCameraBoomLength`
  (params (`increase?` :type Boolean))
  ;[1 1 1] 相机效果
  (if `increase?`
    (bind (_direction _alpha) (`Timeline|时间轴` :!label _label_2) ; 0.5内变化0-1
      (:`Update`
        (set `SpringArmComponent.TargetArmLength` (`KismetMathLibrary.Lerp` 310.0 450.0 _alpha) (`self.SpringArm`)) ; 每帧更新长度
      ))
    (else
      (goto _label_2 :!via `Reverse`))))

(event `EnhancedInput|/Game/Lesson3CtestALL/IA_MZM/IA_Jump_MZM`
  (params (ActionValue :type Boolean) (ElapsedSeconds :type "Float (double-precision)") (TriggeredSeconds :type "Float (double-precision)") (InputAction :type "InputAction Object Reference" :default "/Game/Lesson3CtestALL/IA_MZM/IA_Jump_MZM.IA_Jump_MZM"))
  ;[1 1 1] 跳跃逻辑
  (:`Started`
    (`self.CanTryJump`
      (:`满足跳跃条件`
        (`self.Jump`) ; 芜湖起飞！
      )
      (:`不满足跳跃条件`
        (`self.StopJumping`))))
  (:`Completed`
    (`self.StopJumping`)))

(event `EnhancedInput|/Game/Lesson3CtestALL/IA_MZM/IA_Dodge_MZM`
  (params (ActionValue :type Boolean) (ElapsedSeconds :type "Float (double-precision)") (TriggeredSeconds :type "Float (double-precision)") (InputAction :type "InputAction Object Reference" :default "/Game/Lesson3CtestALL/IA_MZM/IA_Dodge_MZM.IA_Dodge_MZM"))
  (bind _returnvalue (`SkeletalMeshComponent.GetAnimInstance` (`self.Mesh`)))
  ;[1 1 1] 翻滚逻辑
  (:`Completed`
    (`self.CanRoll`
      (:`满足翻滚条件`
        (`AnimInstance.Montage_Stop` _returnvalue 0.1 (`AnimInstance.GetCurrentActiveMontage` _returnvalue)) ; 停止当前蒙太奇播放
        (set `self.isRolling` true) ; 设置翻滚状态
        (`|PlayMontage` (`self.Mesh`) "/Game/Lesson3CtestALL/Anime_MZM/Dodge_MZM/Player_Dodge.Player_Dodge" 1.4) ; 播放翻滚的蒙太奇
      ))))

(event `self.INT_ResetAction`
  ;[1 1 1] 接口实现：重置相关动作
  (set `self.isRolling` false) ; 翻滚重置
  (set `self.isAttacking` false) ; 攻击重置
  (set `self.isHited` false) ; 受击重置
  (`self.End Sprinting`) ; 冲刺重置
)

(event `EnhancedInput|/Game/Lesson3CtestALL/IA_MZM/IA_LAttack`
  (params (ActionValue :type Boolean) (ElapsedSeconds :type "Float (double-precision)") (TriggeredSeconds :type "Float (double-precision)") (InputAction :type "InputAction Object Reference" :default "/Game/Lesson3CtestALL/IA_MZM/IA_LAttack.IA_LAttack"))
  ;[1 1 1] 轻攻击
  (:`Started`
    (`self.CanAttack` "LATK" ; 攻击状态检测
      (:`满足攻击条件`
        (set `self.isAttacking` true) ; 设置攻击状态
        (`|PlayMontage` (`self.Mesh`) (select `int` (`self.LATKCount`) :`0` "/Game/Lesson3CtestALL/Anime_MZM/Attack_MZM/Player_EAttack_1.Player_EAttack_1" :`1` "/Game/Lesson3CtestALL/Anime_MZM/Attack_MZM/Player_EAttack_2.Player_EAttack_2" :`2` "/Game/Lesson3CtestALL/Anime_MZM/Attack_MZM/Player_EAttack_3.Player_EAttack_3" :!type "AnimMontage Object Reference") 1.3 ; 播放攻击蒙太奇
          (:`then`
            (bind _result (`/Engine/EditorBlueprintResources/StandardMacros.IncrementInt` (`self.LATKCount`)) ; 原地递增
              (:`  `
                (if (== _result 3)
                  (set `self.LATKCount` 0) ; 将目录角标重置为0
                )))))))))

(event `self.INT_TraceCheck`
  (params (`Start?` :type Boolean) (DMGMulti :type "Float (double-precision)") (LnockBackPower :type Integer) (Additionalinfo :type "Array of String (by ref)"))
  ;[1 1 1] 接口实现：攻击检测
  (`self.AttributeModifier` DMGMulti) ; 调用伤害计算
  (set `self.knock Back Power` LnockBackPower) ; 击退力（不一定用啊，但先设置了）
  (set `self.Additionalinfo` Additionalinfo) ; 额外信息
  (if `Start?`
    (`self.StartTracing`) ; 开始追踪
    (else
      (`KismetSystemLibrary.K2_ClearTimer` null "TraceChecking") ; 取消每帧执行
    )))

(event `self.INT_HitHandle`
  (params (HitCauser :type "Actor Object Reference") (ReceivedDamage :type "Float (double-precision)") (KnockBackPower :type Integer) (Additionalinfo :type "Array of String (by ref)"))
  (`/Engine/EditorBlueprintResources/StandardMacros.IsValid` HitCauser ; 检测是有伤害制造者
    (:`Is Valid`
      (if (not (`self.isRolling`))
        (set `self.Hit Causer` HitCauser)
        (set `/Game/Lesson3CtestALL/Player_BaseData.CurHP` (`KismetMathLibrary.FClamp` (- (`/Game/Lesson3CtestALL/Player_BaseData.CurHP` (`self.Player_BaseData`)) ReceivedDamage) 0.0 (`/Game/Lesson3CtestALL/Player_BaseData.MaxHP` (`self.Player_BaseData`))) (`self.Player_BaseData`)) ; 一次受击后还剩多少血
        (set `self.isHited` true) ; 现在是受击状态
        (if (<= (`/Game/Lesson3CtestALL/Player_BaseData.CurHP` (`self.Player_BaseData`)) 0.0)
          (`KismetSystemLibrary.PrintString` "Playis Dead")
          (else
            (`KismetSystemLibrary.PrintString` "播放受击表现")
            (set `self.isHited` false) ; 做完表现恢复状态
          ))))))

(event `EnhancedInput|/Game/Lesson3CtestALL/IA_MZM/IA_HAttack`
  (params (ActionValue :type Boolean) (ElapsedSeconds :type "Float (double-precision)") (TriggeredSeconds :type "Float (double-precision)") (InputAction :type "InputAction Object Reference" :default "/Game/Lesson3CtestALL/IA_MZM/IA_HAttack.IA_HAttack"))
  (bind _returnvalue (> (`/Game/Lesson3CtestALL/Player_BaseData.CurSP` (`self.Player_BaseData`)) 0.0))
  ;[1 1 1] 重攻击
  (:`Triggered`
    (if _returnvalue
      (`/Engine/EditorBlueprintResources/StandardMacros.DoOnce` false :!label _label_3 ; 保证Hold的Check只有一次，并在Completed后重置
        (:`Completed`
          (`|PlayMontage` (`self.Mesh`) "/Game/Lesson3CtestALL/Anime_MZM/Attack_MZM/Player_FocusAttack_2.Player_FocusAttack_2" 1.3 0.0 "Attack" ; 跳转到蒙太奇的攻击部分
            (:`OnCompleted`
              (`KismetSystemLibrary.PrintString` "蓄力完毕" true true (struct :`G` 0.66 :`B` 1.0 :`A` 1.0) 3.0)))))))
  (:`Started`
    (if _returnvalue
      (`self.CanAttack` "HATK" ; 攻击状态检测
        (:`满足攻击条件`
          (set `self.isAttacking` true) ; 设置攻击状态
          (`|PlayMontage` (`self.Mesh`) "/Game/Lesson3CtestALL/Anime_MZM/Attack_MZM/Player_FocusAttack_2.Player_FocusAttack_2" 0.95) ; 播放蒙太奇的蓄力部分
        ))))
  (:`Completed`
    (if _returnvalue
      (goto _label_3 :!via `Reset`))))

(event `EnhancedInput|/Game/Lesson3CtestALL/IA_MZM/IA_Test_MZM`
  (params (ActionValue :type Boolean) (ElapsedSeconds :type "Float (double-precision)") (TriggeredSeconds :type "Float (double-precision)") (InputAction :type "InputAction Object Reference" :default "/Game/Lesson3CtestALL/IA_MZM/IA_Test_MZM.IA_Test_MZM"))
  (:`Triggered`
    (`/Engine/EditorBlueprintResources/StandardMacros.DoOnce` false :!label _label_4 ; 保证Hold的Check只有一次，并在Completed后重置
      (:`Completed`
        (`KismetSystemLibrary.PrintString` "Trigger" true true (struct :`R` 1.0 :`G` 0.882116 :`A` 1.0) 1.0))))
  (:`Started`
    (`KismetSystemLibrary.PrintString` "Start" true true (struct :`R` 1.0 :`B` 0.04617 :`A` 1.0) 4.0))
  (:`Ongoing`
    (`KismetSystemLibrary.PrintString` "ongoing" true true (struct :`R` 0.260844 :`B` 1.0 :`A` 1.0) 1.0))
  (:`Canceled`
    (`KismetSystemLibrary.PrintString` "Canceled" true true (struct :`G` 0.66 :`B` 1.0 :`A` 1.0) 1.0))
  (:`Completed`
    (`KismetSystemLibrary.PrintString` "Completed" true true (struct :`G` 1.0 :`B` 0.022493 :`A` 1.0) 4.0)
    (goto _label_4 :!via `Reset`)))

(fn `AttributeModifier`
  (params (DMGMulti :type "Float (double-precision)"))
  (bind _output_get (set `self.DMGMulti` DMGMulti)) ; 赋值伤害倍率
  (set `self.FinalDamage` (* _output_get (`/Game/Lesson3CtestALL/Player_BaseData.BaseATK` (`self.Player_BaseData`)))) ; 设置最终伤害
  (return))

(fn `End Sprinting`
  (set `CharacterMovementComponent.MaxWalkSpeed` 600.0 (`self.CharacterMovement`)) ; 设置最大速度
  (message `/Game/Lesson3CtestALL/BPI/BPI_Anime.INT_SetPlayRate` (`SkeletalMeshComponent.GetAnimInstance` (`self.Mesh`)) 1.0) ; 调用接口去设置播放速率
  (set `self.isSprinting` false) ; 记录玩家处于非冲刺状态
  (`self.ChangeCameraBoomLength` false) ; 缩短相机臂
)

(fn `HandleSP`
  (params (ActionName :type String))
  (bind _output_get (set `/Game/Lesson3CtestALL/Player_BaseData.CurSP` (`KismetMathLibrary.FClamp` (+ (`/Game/Lesson3CtestALL/Player_BaseData.CurSP` (`self.Player_BaseData`)) (`BlueprintMapLibrary.Map_Find` (`self.SPcost`) ActionName)) 0.0 (`/Game/Lesson3CtestALL/Player_BaseData.MaxSP` (`self.Player_BaseData`))) (`self.Player_BaseData`)))
  (`KismetSystemLibrary.PrintString` (`KismetStringLibrary.Conv_DoubleToString` _output_get) true true (struct :`G` 1.0 :`B` 0.041187 :`A` 1.0) 3.0))

(fn `INT_GetStatus`
  (returns (`Live?` :type Boolean) (Hitted :type Boolean))
  (return false false))

(fn `RetrieveMontageFromString`
  (params (AnimStr :type String))
  (returns (Montage :type "AnimInstance Object Reference"))
  (return null))

(fn `Start Sprinting`
  (set `CharacterMovementComponent.MaxWalkSpeed` 800.0 (`self.CharacterMovement`)) ; 设置最大速度
  (message `/Game/Lesson3CtestALL/BPI/BPI_Anime.INT_SetPlayRate` (`SkeletalMeshComponent.GetAnimInstance` (`self.Mesh`)) 1.5) ; 调用接口去设置播放速率
  (set `self.isSprinting` true) ; 记录玩家处于冲刺状态
  (`self.ChangeCameraBoomLength` true) ; 伸长相机臂
)

(fn `StartTracing`
  ;[1 1 1] 清空上一帧的插槽坐标和受击对象
  (`KismetArrayLibrary.Array_Clear` (`self.TracePointLocations`))
  (`KismetArrayLibrary.Array_Clear` (`self.HitActorsInOneShoot`))
  ;[1 1 1] 遍历当前帧所有插槽
  (bind _returnvalue (`GameplayStatics.GetActorOfClass` "/Game/Lesson3CtestALL/Weapon/BP_MyGreatSword_00.BP_MyGreatSword_00_C")) ; 获取武器蓝图类
  (bind _staticmesh (`/Game/Lesson3CtestALL/Weapon/BP_MyGreatSword_00.StaticMesh` _returnvalue))
  (for _array_element (`SceneComponent.GetAllSocketNames` _staticmesh)
    ;[1 1 1] 存放插槽坐标到数组内
    (`KismetArrayLibrary.Array_Add` (`self.TracePointLocations`) (`SceneComponent.GetSocketLocation` _staticmesh _array_element)))
  ;[1 1 1] 每帧重新遍历
  (`KismetSystemLibrary.K2_SetTimer` null "TraceChecking" (`GameplayStatics.GetWorldDeltaSeconds`) true) ; 每帧执行的计时器，即每帧都更新
)

(fn `TraceChecking`
  ;[1 1 1] 获取武器插槽并每帧检测
  (bind _returnvalue (`GameplayStatics.GetActorOfClass` "/Game/Lesson3CtestALL/Weapon/BP_MyGreatSword_00.BP_MyGreatSword_00_C")) ; 获取武器蓝图类
  (bind _staticmesh (`/Game/Lesson3CtestALL/Weapon/BP_MyGreatSword_00.StaticMesh` _returnvalue))
  (for (_array_element _array_index) (`SceneComponent.GetAllSocketNames` _staticmesh)
    (bind _returnvalue_2 (`SceneComponent.GetSocketLocation` _staticmesh _array_element))
    (bind _outhits (`KismetSystemLibrary.SphereTraceMultiForObjects` :`Start` (`|GetArrayItem` (`self.TracePointLocations`) _array_index) :`End` _returnvalue_2 :`Radius` 15.0 :`ObjectTypes` (`|MakeArray` "ObjectTypeQuery3" :!type "EObjectTypeQuery Enum") :`DrawDebugType` "ForDuration")) ; 每帧检测受击物体
    ;[1 1 1] 根据数组内是否存在受击对象进行打印
    (for _array_element_2 _outhits
      (bind (_bblockinghit _binitialoverlap _time _distance _location _impactpoint _normal _impactnormal _physmat _hitactor) (`GameplayStatics.BreakHitResult` _array_element_2))
      (`/Engine/EditorBlueprintResources/StandardMacros.IsValid` _hitactor ; 检测是否存在受击结果
        (:`Is Valid`
          (if (not (`KismetArrayLibrary.Array_Contains` (`self.HitActorsInOneShoot`) _hitactor))
            (`KismetArrayLibrary.Array_AddUnique` (`self.HitActorsInOneShoot`) _hitactor) ; 不是，则将其加入受击对象数组
            (`KismetSystemLibrary.PrintString` (`KismetSystemLibrary.GetDisplayName` _hitactor) true true (struct :`R` 1.0 :`G` 0.087137 :`A` 1.0) 8.0) ; 并打印一次受击结果
            (message `/Game/M_Enemy/BPI_Combat.INT_HitHandle` _hitactor self (`self.FinalDamage`) (`self.knock Back Power`) (`self.Additionalinfo`))))))
    ;[1 1 1] 将上一帧的内容更新为当前帧
    (`KismetArrayLibrary.Array_Set` (`self.TracePointLocations`) _array_index _returnvalue_2)))

(fn `UserConstructionScript`)