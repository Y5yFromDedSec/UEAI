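; Stage 2 player character Blueprint for a third-person action game, covering movement, camera, sprint, jump, dodge and attacks via Enhanced Input.
; Gate functions check state flags and, for dodge and attacks, stamina costs, which are not deducted here; INTResetAction clears the action flags.
; Montages drive a three-step light combo and charged heavy attack, while sprinting adjusts speed, anim rate and boom length.
; Debug keys test enemy AI states, noise and damage sensing.
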(event `self.ReceiveBeginPlay`
  (set `self.CurSP` (`self.MaxSP`)))

(event `self.ReceiveActorBeginOverlap`
  (params (OtherActor :type "Actor Object Reference")))

(event `Key|M`
  (params (Key :type "Key Structure"))
  ;[1 1 1] AI验证模块
  (:`Pressed`
    (`KismetSystemLibrary.PrintString` "改变AI状态") ; Debug
    (bind _returnvalue (`GameplayStatics.GetActorOfClass` "/Game/M_Enemy/BP_EnemyBase_MZM.BP_EnemyBase_MZM_C")) ; 获取Actor类
    (bind _asaic_enemy_base_mzm (cast `/Game/M_Enemy/AI/AIC_Enemy_Base_MZM` (`AIBlueprintHelperLibrary.GetAIController` _returnvalue))) ; 将AIC转化为我们的AIC
    (`/Engine/EditorBlueprintResources/StandardMacros.FlipFlop` ; 翻转！
      (:`A`
        (`/Game/M_Enemy/AI/AIC_Enemy_Base_MZM.SetStatesAsPassive` _asaic_enemy_base_mzm) ; 切换为Passive
      )
      (:`B`
        (`/Game/M_Enemy/AI/AIC_Enemy_Base_MZM.SetStatesAsAttack` _asaic_enemy_base_mzm self) ; 切换为Attack
      ))))

(event `EnhancedInput|/Game/Lesson3CtestALL/IA_MZM/IA_Move_MZM`
  (params (ActionValue :type "Vector2D Structure") (ElapsedSeconds :type "Float (double-precision)") (TriggeredSeconds :type "Float (double-precision)") (InputAction :type "InputAction Object Reference" :default "/Game/Lesson3CtestALL/IA_MZM/IA_Move_MZM.IA_Move_MZM"))
  (bind (_returnvalue_roll _returnvalue_pitch _returnvalue_yaw) (`KismetMathLibrary.BreakRotator` (`self.GetControlRotation`)))
  (bind (_x _y) (`KismetMathLibrary.BreakVector2D` ActionValue))
  ;[1 1 1] 玩家角色移动
  (:`Triggered`
    (set `self.OriginForward` _x) ; 当按下移动键时设置初始前进方向
    (set `self.OriginRight` _y) ; 当按下移动键时设置初始右进方向
    (`self.AddMovementInput` (`KismetMathLibrary.GetForwardVector` (`KismetMathLibrary.MakeRotator` 0.0 0.0 _returnvalue_yaw)) (`self.OriginForward`)) ; WS控制前进后退
    (`self.AddMovementInput` (`KismetMathLibrary.GetRightVector` (`KismetMathLibrary.MakeRotator` 0.0 0.0 _returnvalue_yaw)) (`self.OriginRight`)) ; AD控制左右移动
  )
  (:`Canceled`
    (set `self.OriginForward` 0.0 :!label _label) ; 当完成or取消时将初始前进方向设置为0
    (set `self.OriginRight` 0.0) ; 当完成or取消时将初始右进方向设置为0
  )
  (:`Completed`
    (goto _label)))

(event `self.ReceiveTick`
  (params (DeltaSeconds :type "Float (single-precision)")))

(event `Key|N`
  (params (Key :type "Key Structure"))
  (bind _returnvalue (`self.K2_GetActorLocation`))
  ;[1 1 1] AI验证模块
  (:`Pressed`
    (`self.MakeNoise` 1.0 self _returnvalue)
    (`GameplayStatics.SpawnEmitterAtLocation` "/Game/StarterContent/Particles/P_Explosion.P_Explosion" _returnvalue)
    (`GameplayStatics.PlaySoundAtLocation` "/Game/StarterContent/Audio/Explosion01.Explosion01" _returnvalue (struct) 1.0 1.0 0.0 null null null null)))

(event `EnhancedInput|/Game/Lesson3CtestALL/IA_MZM/IA_CameraControl_MZM`
  (params (ActionValue :type "Vector2D Structure") (ElapsedSeconds :type "Float (double-precision)") (TriggeredSeconds :type "Float (double-precision)") (InputAction :type "InputAction Object Reference" :default "/Game/Lesson3CtestALL/IA_MZM/IA_CameraControl_MZM.IA_CameraControl_MZM"))
  (bind (_x _y) (`KismetMathLibrary.BreakVector2D` ActionValue))
  ;[1 1 1] 相机控制
  (:`Triggered`
    (`self.AddControllerYawInput` _x) ; X为屏幕横轴，控制水平方向
    (`self.AddControllerPitchInput` (* _y -1.0)) ; Y轴为屏幕竖轴，控制垂直方向
  ))

(event `Key|X`
  (params (Key :type "Key Structure"))
  ;[1 1 1] AI验证模块
  (:`Pressed`
    (bind _returnvalue (`GameplayStatics.GetActorOfClass` "/Game/M_Enemy/BP_EnemyBase_MZM.BP_EnemyBase_MZM_C"))
    (`AISense_Damage.ReportDamageEvent` _returnvalue self 0.0 (`self.K2_GetActorLocation`))))

(event `EnhancedInput|/Game/Lesson3CtestALL/IA_MZM/IA_Sprint_MZM`
  (params (ActionValue :type Boolean) (ElapsedSeconds :type "Float (double-precision)") (TriggeredSeconds :type "Float (double-precision)") (InputAction :type "InputAction Object Reference" :default "/Game/Lesson3CtestALL/IA_MZM/IA_Sprint_MZM.IA_Sprint_MZM"))
  ;[1 1 1] 冲刺逻辑
  (:`Triggered`
    (`self.CanSprinting` ElapsedSeconds ; 冲刺的状态判断
      (:`满足冲刺`
        (`self.Start Sprinting`) ; 我他妈来了
      )
      (:`不满足冲刺`
        (`self.End Sprinting`) ; 萎了
      )))
  (:`Completed`
    (if (`self.isSprinting`)
      (`self.End Sprinting`) ; 萎了
    )))

(event `ChangeCameraBoomLength`
  (params (`increase?` :type Boolean))
  ;[1 1 1] 相机效果
  (if `increase?`
    (bind (_direction _alpha) (`Timeline|时间轴` :!label _label_2) ; 0.5内变化0-1
      (:`Update`
        (set `SpringArmComponent.TargetArmLength` (`KismetMathLibrary.Lerp` 310.0 450.0 _alpha) (`self.SpringArm`)) ; 每帧更新长度
      ))
    (else
      (goto _label_2 :!via `Reverse`))))

(event `EnhancedInput|/Game/Lesson3CtestALL/IA_MZM/IA_Jump_MZM`
  (params (ActionValue :type Boolean) (ElapsedSeconds :type "Float (double-precision)") (TriggeredSeconds :type "Float (double-precision)") (InputAction :type "InputAction Object Reference" :default "/Game/Lesson3CtestALL/IA_MZM/IA_Jump_MZM.IA_Jump_MZM"))
  ;[1 1 1] 跳跃逻辑
  (:`Started`
    (`self.CanTryJump`
      (:`满足跳跃条件`
        (`self.Jump`) ; 芜湖起飞！
      )
      (:`不满足跳跃条件`
        (`self.StopJumping`))))
  (:`Completed`
    (`self.StopJumping`)))

(event `EnhancedInput|/Game/Lesson3CtestALL/IA_MZM/IA_Dodge_MZM`
  (params (ActionValue :type Boolean) (ElapsedSeconds :type "Float (double-precision)") (TriggeredSeconds :type "Float (double-precision)") (InputAction :type "InputAction Object Reference" :default "/Game/Lesson3CtestALL/IA_MZM/IA_Dodge_MZM.IA_Dodge_MZM"))
  (bind _returnvalue (`SkeletalMeshComponent.GetAnimInstance` (`self.Mesh`)))
  ;[1 1 1] 翻滚逻辑
  (:`Completed`
    (`self.CanRoll`
      (:`满足翻滚条件`
        (`AnimInstance.Montage_Stop` _returnvalue 0.1 (`AnimInstance.GetCurrentActiveMontage` _returnvalue)) ; 停止当前蒙太奇播放
        (set `self.isRolling` true) ; 设置翻滚状态
        (`self.PlayAnimMontage` "/Game/Lesson3CtestALL/Anime_MZM/Dodge_MZM/Player_Dodge.Player_Dodge")))))

(event `/Game/Lesson3CtestALL/BPI/BPI_Notify.INT_ResetAction`
  ;[1 1 1] 重置相关动作
  (set `self.isRolling` false) ; 翻滚重置
  (set `self.isAttacking` false) ; 攻击重置
  (set `self.isHited` false) ; 受击重置
  (`self.End Sprinting`) ; 冲刺重置
)

(event `EnhancedInput|/Game/Lesson3CtestALL/IA_MZM/IA_LAttack`
  (params (ActionValue :type Boolean) (ElapsedSeconds :type "Float (double-precision)") (TriggeredSeconds :type "Float (double-precision)") (InputAction :type "InputAction Object Reference" :default "/Game/Lesson3CtestALL/IA_MZM/IA_LAttack.IA_LAttack"))
  ;[1 1 1] 轻攻击
  (:`Started`
    (`self.CanAttack` "LATK" ; 攻击状态检测
      (:`满足攻击条件`
        (set `self.isAttacking` true) ; 设置攻击状态
        (`|PlayMontage` (`self.Mesh`) (select `int` (`self.LATKCount`) :`0` "/Game/Lesson3CtestALL/Anime_MZM/Attack_MZM/Player_Attack_1.Player_Attack_1" :`1` "/Game/Lesson3CtestALL/Anime_MZM/Attack_MZM/Player_Attack_2.Player_Attack_2" :`2` "/Game/Lesson3CtestALL/Anime_MZM/Attack_MZM/Player_Attack_3.Player_Attack_3" :!type "AnimMontage Object Reference") 1.3 ; 播放攻击蒙太奇
          (:`then`
            (bind _result (`/Engine/EditorBlueprintResources/StandardMacros.IncrementInt` (`self.LATKCount`)) ; 原地递增
              (:`  `
                (if (== _result 3)
                  (set `self.LATKCount` 0) ; 将目录角标重置为0
                )))))))))

(event `EnhancedInput|/Game/Lesson3CtestALL/IA_MZM/IA_HAttack`
  (params (ActionValue :type Boolean) (ElapsedSeconds :type "Float (double-precision)") (TriggeredSeconds :type "Float (double-precision)") (InputAction :type "InputAction Object Reference" :default "/Game/Lesson3CtestALL/IA_MZM/IA_HAttack.IA_HAttack"))
  (:`Triggered`
    (`/Engine/EditorBlueprintResources/StandardMacros.DoOnce` false :!label _label_3 ; 保证Hold的Check只有一次，并在Completed后重置
      (:`Completed`
        (`|PlayMontage` (`self.Mesh`) "/Game/Lesson3CtestALL/Anime_MZM/Attack_MZM/Player_FocusAttack_2.Player_FocusAttack_2" 1.5 0.0 "Attack" ; 跳转到蒙太奇的攻击部分
          (:`then`
            (`KismetSystemLibrary.PrintString` "蓄力完毕" true true (struct :`G` 0.66 :`B` 1.0 :`A` 1.0) 3.0))))))
  (:`Started`
    (`self.CanAttack` "HATK" ; 攻击状态检测
      (:`满足攻击条件`
        (set `self.isAttacking` true) ; 设置攻击状态
        (`|PlayMontage` (`self.Mesh`) "/Game/Lesson3CtestALL/Anime_MZM/Attack_MZM/Player_FocusAttack_2.Player_FocusAttack_2" 0.95) ; 播放蒙太奇的蓄力部分
      )))
  (:`Completed`
    (goto _label_3 :!via `Reset`)))

(event `EnhancedInput|/Game/Lesson3CtestALL/IA_MZM/IA_Test_MZM`
  (params (ActionValue :type Boolean) (ElapsedSeconds :type "Float (double-precision)") (TriggeredSeconds :type "Float (double-precision)") (InputAction :type "InputAction Object Reference" :default "/Game/Lesson3CtestALL/IA_MZM/IA_Test_MZM.IA_Test_MZM"))
  (:`Triggered`
    (`KismetSystemLibrary.PrintString` "Trigger" true true (struct :`R` 1.0 :`G` 0.882116 :`A` 1.0) 1.0))
  (:`Started`
    (`KismetSystemLibrary.PrintString` "Start" true true (struct :`R` 1.0 :`B` 0.04617 :`A` 1.0) 4.0))
  (:`Ongoing`
    (`KismetSystemLibrary.PrintString` "ongoing" true true (struct :`R` 0.260844 :`B` 1.0 :`A` 1.0) 1.0))
  (:`Canceled`
    (`KismetSystemLibrary.PrintString` "Canceled" true true (struct :`G` 0.66 :`B` 1.0 :`A` 1.0) 1.0))
  (:`Completed`
    (`KismetSystemLibrary.PrintString` "Completed" true true (struct :`G` 1.0 :`B` 0.022493 :`A` 1.0) 4.0)))

(fn `End Sprinting`
  (set `CharacterMovementComponent.MaxWalkSpeed` 600.0 (`self.CharacterMovement`)) ; 设置最大速度
  (message `/Game/Lesson3CtestALL/BPI/BPI_Anime.INT_SetPlayRate` (`SkeletalMeshComponent.GetAnimInstance` (`self.Mesh`)) 1.0) ; 调用接口去设置播放速率
  (set `self.isSprinting` false) ; 记录玩家处于非冲刺状态
  (`self.ChangeCameraBoomLength` false) ; 缩短相机臂
)

(fn `RetrieveMontageFromString`
  (params (AnimStr :type String))
  (returns (Montage :type "AnimInstance Object Reference"))
  (return null))

(fn `Start Sprinting`
  (set `CharacterMovementComponent.MaxWalkSpeed` 800.0 (`self.CharacterMovement`)) ; 设置最大速度
  (message `/Game/Lesson3CtestALL/BPI/BPI_Anime.INT_SetPlayRate` (`SkeletalMeshComponent.GetAnimInstance` (`self.Mesh`)) 1.5) ; 调用接口去设置播放速率
  (set `self.isSprinting` true) ; 记录玩家处于冲刺状态
  (`self.ChangeCameraBoomLength` true) ; 伸长相机臂
)

(fn `UserConstructionScript`)