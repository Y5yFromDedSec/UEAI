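; Base enemy character that fights the player with a sword and montage attack, tracks HP in a widget and is destroyed at zero HP.
; Attack checks sphere-overlap ahead of it and send scaled damage to "Player"-tagged actors through a hit interface.
; Incoming hits use that interface to reduce HP, report AI damage sense events and update the bar.
; Getters and a speed setter expose combat ranges, patrol route, status and movement tiers.
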(event `self.ReceiveBeginPlay`
  (set `self.EnemyCurHP` (`self.EnemyMaxHP`))
  (bind _asui_enemy_hp (cast `/Game/M_UI/UI_EnemyHP` (`WidgetComponent.GetUserWidgetObject` (`self.HPbar`))))
  (bind _output_get (set `self.As UI Enemy HP` _asui_enemy_hp))
  (`/Game/M_UI/UI_EnemyHP.UpdateHP` _output_get (`self.EnemyCurHP`) (`self.EnemyMaxHP`)))

(event `/Game/M_Enemy/BPI_EnemyAI.Attack`
  (`KismetSystemLibrary.PrintString` "播放攻击蒙太奇！") ; debug一下，后面记得自己删了
  (`|PlayMontage` (`self.Mesh`) "/Game/M_Enemy/EnemyAnime/Melee/Enemy_Combo.Enemy_Combo" 1.3 ; 播放攻击蒙太奇
    (:`OnCompleted`
      _)
    (:`OnInterrupted`
      _))
  (`self.OnAttackEnd`) ; 调用事件
)

(event `Sword`
  (bind _returnvalue (`|SpawnActorFromClass` "/Game/M_Enemy/Weapon/BP_Sword.BP_Sword_C" (`self.GetTransform`) "Undefined" "MultiplyWithRoot" null null))
  (`self.K2_AttachToComponent` _returnvalue (`self.Mesh`) "Enemy_Sword_R" "SnapToTarget" "SnapToTarget" "SnapToTarget" true))

(event `/Game/M_Enemy/BPI_Combat.INT_HitHandle`
  (params (HitCauser :type "Actor Object Reference") (ReceivedDamage :type "Float (double-precision)") (KnockBackPower :type Integer) (Additionalinfo :type "Array of String (by ref)"))
  (bind _as_ui_enemy_hp (`self.As UI Enemy HP`))
  (set `self.Hit Causer` HitCauser) ; 设置攻击造成者
  (set `self.Received Damage` ReceivedDamage) ; 设置受到的攻击
  (set `self.RecivedKnockBackPower` KnockBackPower) ; 设置受到的击退力
  (set `self.ReceivedAdditionalinfo` Additionalinfo) ; 设置收到的额外信息
  (if (not (`self.isDead`))
    (bind _output_get (set `self.EnemyCurHP` (- (`self.EnemyCurHP`) (`self.Received Damage`)))) ; 赋给当前HP
    (`KismetSystemLibrary.PrintString` (`KismetStringLibrary.Conv_DoubleToString` _output_get)) ; 打印下血量看看
    (if (<= _output_get 0.0)
      (set `self.isDead` true) ; 设置死亡状态
      (`self.K2_DestroyActor`) ; 死亡则销毁目标
      (`KismetSystemLibrary.PrintString` "EnemyDie!")
      (else
        (bind _output_get_2 (set `self.isHit` true)) ; 设置受击状态
        (`AISense_Damage.ReportDamageEvent` self (`GameplayStatics.GetPlayerPawn` 0))
        (`Widget.SetVisibility` _as_ui_enemy_hp (select `bool` _output_get_2 :`false` "Hidden" :`true` "Visible" :!type "ESlateVisibility Enum"))
        (`/Game/M_UI/UI_EnemyHP.UpdateHP` _as_ui_enemy_hp (`self.EnemyCurHP`) (`self.EnemyMaxHP`))))))

(event `/Game/M_Enemy/BPI_Combat.INT_EnemyAttackCheck`
  (params (CenterDis :type "Float (double-precision)") (SphereRas :type "Float (double-precision)") (DamageRatio :type "Float (double-precision)") (Additionalinfo :type "Array of String (by ref)"))
  (bind _returnvalue (+ (`self.K2_GetActorLocation`) (* (`self.GetActorForwardVector`) CenterDis)))
  (set `self.AttackCheckAdditionalinfo` Additionalinfo) ; 提升自定义变量
  (set `self.EnemyDamage Ratio` DamageRatio) ; 提升自定义变量
  (`|ExecutionSequence`
    (:`then_0`
      (bind _outactors (`KismetSystemLibrary.SphereOverlapActors` _returnvalue SphereRas (`|MakeArray` "ObjectTypeQuery3" :!type "EObjectTypeQuery Enum") null (`|MakeArray` self :!type "Actor Object Reference"))) ; 检测球形重叠
      (for _array_element _outactors
        (if (and (`self.ActorHasTag` _array_element "Player") (not (`KismetArrayLibrary.Array_Contains` (`self.DamageTheActor`) _array_element)))
          (`KismetArrayLibrary.Array_AddUnique` (`self.DamageTheActor`) _array_element) ; 是的话，则添加进去，防止二次伤害
          (message `/Game/M_Enemy/BPI_Combat.INT_HitHandle` _array_element self (* (`self.EnemyBaseDamage`) (`self.EnemyDamage Ratio`)) 0 (`self.AttackCheckAdditionalinfo`)) ; 传递给HitHandle接口，后续这个接口也需要挂接到BP_Player
        ))
      (`KismetArrayLibrary.Array_Clear` (`self.DamageTheActor`)) ; 重置清空
    )
    (:`then_1`
      (`KismetSystemLibrary.DrawDebugSphere` _returnvalue SphereRas 24 (struct :`R` 1.0 :`G` 1.0 :`B` 1.0 :`A` 1.0) 8.0 3.0) ; debug信息
    )))

(fn `GetIdealRange`
  (returns (AttackRadius :type "Float (double-precision)") (DefendRadius :type "Float (double-precision)"))
  (return 150.0 350.0))

(fn `GetPartolRoute`
  (returns (m_PatrolRoute :type "/Game/M_Enemy/BP_PatrolRoute Object Reference"))
  (return (`self.PatrolRoute`)))

(fn `HandleHitedVFX`
  (`GameplayStatics.SpawnEmitterAtLocation` "/Game/StarterContent/Particles/P_Smoke.P_Smoke" (`self.K2_GetActorLocation`) (`KismetMathLibrary.MakeRotator` 0.0 0.0 (`KismetMathLibrary.RandomFloatInRange` -180.0 180.0))))

(fn `INT_GetStatus`
  (returns (`Live?` :type Boolean) (Hitted :type Boolean))
  (return (not (`self.isDead`)) false))

(fn `SetMovementSpeed`
  (params (Speed :type "/Game/M_Enemy/Enum/E_MovementSpeedSet Enum" :default "NewEnumerator0"))
  (returns (SpeedValue :type "Float (double-precision)"))
  (bind _output_get (set `CharacterMovementComponent.MaxWalkSpeed` (select `/Game/M_Enemy/Enum/E_MovementSpeedSet` Speed :`NewEnumerator1` 250.0 :`NewEnumerator2` 450.0 :`NewEnumerator3` 550.0 :!type "Float (single-precision)") (`self.CharacterMovement`))) ; 将速度设给当前的移动
  (return _output_get) ; 返回该数值给移动组件
)

(fn `UserConstructionScript`)