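; Melee enemy Blueprint that equips a sword and performs a great-sword combo attack.
; The Sword event spawns BP_Sword and snaps it to the right-hand sword socket on the mesh.
; The Attack event plays the combo montage slightly sped up, then calls OnAttackEnd whether it completes or is interrupted.
; BeginPlay is empty, with its parent call disabled, and a debug print remains in Attack.
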(event `self.ReceiveBeginPlay`)

(event `/Game/M_Enemy/BPI_EnemyAI.Attack`
  (`KismetSystemLibrary.PrintString` "播放攻击蒙太奇！") ; debug一下，后面记得自己删了
  (`|PlayMontage` (`self.Mesh`) "/Game/GreatSword/GreatSword/Battle/Root/Combo_Sample/GreatSword_Combo1.GreatSword_Combo1" 1.3 ; 播放攻击蒙太奇
    (:`OnCompleted`
      _)
    (:`OnInterrupted`
      _))
  (`self.OnAttackEnd`) ; 调用事件
)

(event `Sword`
  (bind _returnvalue (`|SpawnActorFromClass` "/Game/M_Enemy/Weapon/BP_Sword.BP_Sword_C" (`self.GetTransform`) "Undefined" "MultiplyWithRoot" null null))
  (`self.K2_AttachToComponent` _returnvalue (`self.Mesh`) "Enemy_Sword_R" "SnapToTarget" "SnapToTarget" "SnapToTarget" true))

(fn `UserConstructionScript`
  (`parent.UserConstructionScript`))