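; Ranged enemy Blueprint that dual-wields guns and fires projectiles at the Stage 4 player.
; BeginPlay attaches a gun to each hand socket and caches the player as AttackTarget.
; Attack plays a montage whose notify spawns an Arrow toward the target, then signals attack end on completion or interruption.
; Impact damages the hit actor but always sends the hit callback to AttackTarget; the inherited attack check is overridden empty.
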(event `self.Attack`
  (`|PlayMontage` (`self.Mesh`) "/Game/M_Enemy/EnemyAnime/Ranged/RangedAttack_Enemy.RangedAttack_Enemy" 1.3 ; 播放攻击蒙太奇
    (:`OnCompleted`
      (`self.OnAttackEnd` :!label _label) ; 调用事件
    )
    (:`OnInterrupted`
      (goto _label))
    (:`OnNotifyBegin`
      (bind _returnvalue (`|SpawnActorFromClass` "/Game/M_Bullet/Arrow.Arrow_C" (`SceneComponent.K2_GetComponentToWorld` (`self.Scene`)) "Undefined" "MultiplyWithRoot" self 1000.0 0.05 (`self.AttackTarget`) false null))
      (add `/Game/M_Bullet/Bullet_Base.OnBulletImpact` _returnvalue (delegate `OnBulletImpact_事件`))
      (`PrimitiveComponent.IgnoreActorWhenMoving` (`self.CapsuleComponent`) _returnvalue true))))

(event `self.ReceiveBeginPlay`
  (`parent.ReceiveBeginPlay`)
  (`self.Gun`)
  (`self.GUn2`)
  (bind _returnvalue (`GameplayStatics.GetActorOfClass` "/Game/Lesson3CtestALL/BP_Player_MZM_Stage4.BP_Player_MZM_Stage4_C"))
  (set `self.AttackTarget` _returnvalue))

(event `OnBulletImpact_事件`
  (params (`Other Actor` :type "Actor Object Reference") (Hit :type "HitResult Structure"))
  (bind _returnvalue (`GameplayStatics.ApplyDamage` (`.HitActor` (`GameplayStatics.BreakHitResult` Hit)) (`self.EnemyBaseDamage`) null self))
  (`/Game/M_Enemy/BPI_Combat.INT_HitHandle` :`self` (`self.AttackTarget`) :`HitCauser` self :`ReceivedDamage` _returnvalue))

(event `self.INT_HitHandle`
  (params (HitCauser :type "Actor Object Reference") (ReceivedDamage :type "Float (double-precision)") (KnockBackPower :type Integer) (Additionalinfo :type "Array of String (by ref)"))
  (`parent.INT_HitHandle` HitCauser ReceivedDamage KnockBackPower Additionalinfo))

(event `Gun`
  (bind _returnvalue (`|SpawnActorFromClass` "/Game/M_Enemy/Weapon/BP_Gun.BP_Gun_C" (`self.GetTransform`) "Undefined" "MultiplyWithRoot" null null))
  (`self.K2_AttachToComponent` _returnvalue (`self.Mesh`) "hand_rSocket" "SnapToTarget" "SnapToTarget" "SnapToTarget" true))

(event `self.INT_EnemyAttackCheck`
  (params (CenterDis :type "Float (double-precision)") (SphereRas :type "Float (double-precision)") (DamageRatio :type "Float (double-precision)") (Additionalinfo :type "Array of String (by ref)")))

(event `GUn2`
  (bind _returnvalue (`|SpawnActorFromClass` "/Game/M_Enemy/Weapon/BP_Gun.BP_Gun_C" (`self.GetTransform`) "Undefined" "MultiplyWithRoot" null null))
  (`self.K2_AttachToComponent` _returnvalue (`self.Mesh`) "hand_lSocket" "SnapToTarget" "SnapToTarget" "SnapToTarget" true))

(fn `UserConstructionScript`
  (`parent.UserConstructionScript`))