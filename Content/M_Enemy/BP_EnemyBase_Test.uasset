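; BP_EnemyBase_Test is a test base enemy character with a health bar widget, a greatsword attack and getters for movement and patrol behavior.
; BeginPlay initializes the HP widget, and the Sword event spawns BP_Sword onto the right-hand mesh socket.
; Attack plays a combo montage and calls OnAttackEnd on completion or interruption.
; Functions supply attack and defend radii, return the patrol route, and map a speed enum to max walk speed.
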(event `self.ReceiveBeginPlay`
  (bind _asui_hp (cast `/Game/M_Enemy/UI/UI_HP` (`WidgetComponent.GetUserWidgetObject` (`self.HP`))))
  (bind _output_get (set `self.UI_HP` _asui_hp))
  (`/Game/M_Enemy/UI/UI_HP.UpdateHP` _output_get 0.1 1.0))

(event `self.Attack`
  (`KismetSystemLibrary.PrintString` "播放攻击蒙太奇！") ; debug一下，后面记得自己删了
  (`|PlayMontage` (`self.Mesh`) "/Game/GreatSword/GreatSword/Battle/Root/Combo_Sample/GreatSword_Combo2.GreatSword_Combo2" 1.3 ; 播放攻击蒙太奇
    (:`OnCompleted`
      _)
    (:`OnInterrupted`
      _))
  (`self.OnAttackEnd`) ; 调用事件
)

(event `Sword`
  (bind _returnvalue (`|SpawnActorFromClass` "/Game/M_Enemy/Weapon/BP_Sword.BP_Sword_C" (`self.GetTransform`) "Undefined" "MultiplyWithRoot" null null))
  (`self.K2_AttachToComponent` _returnvalue (`self.Mesh`) "Enemy_Sword_R" "SnapToTarget" "SnapToTarget" "SnapToTarget" true))

(fn `GetIdealRange`
  (returns (AttackRadius :type "Float (double-precision)") (DefendRadius :type "Float (double-precision)"))
  (return 150.0 350.0))

(fn `GetPartolRoute`
  (returns (m_PatrolRoute :type "/Game/M_Enemy/BP_PatrolRoute Object Reference"))
  (return (`self.PatrolRoute`)))

(fn `SetMovementSpeed`
  (params (Speed :type "/Game/M_Enemy/Enum/E_MovementSpeedSet Enum" :default "NewEnumerator0"))
  (returns (SpeedValue :type "Float (double-precision)"))
  (bind _output_get (set `CharacterMovementComponent.MaxWalkSpeed` (select `/Game/M_Enemy/Enum/E_MovementSpeedSet` Speed :`NewEnumerator1` 250.0 :`NewEnumerator2` 450.0 :`NewEnumerator3` 550.0 :!type "Float (single-precision)") (`self.CharacterMovement`))) ; 将速度设给当前的移动
  (return _output_get) ; 返回该数值给移动组件
)

(fn `UserConstructionScript`)